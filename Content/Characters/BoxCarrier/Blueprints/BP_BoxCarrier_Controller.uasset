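; Player controller for the BoxCarrier character that handles click-to-move and toggling of option widgets on world actors.
; Left click sends the cursor hit location to the pawn as a move message, sprinting on a double tap timed from the previous release.
; Right click traces under the cursor and calls ToggleVisibility on actors implementing BPI_CanToggle.
; Both clicks first hide all "Options" widgets on actors tagged "CanToggle".
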(event EventBeginPlay
  (bind _asbp_box_carrier (Utilities|Casting|CastToBP_BoxCarrier (Game|Player|GetPlayerPawn 0)))
  (Variables|Default|SetBox%20Carrier _asbp_box_carrier))

(event EventTick
  (params (DeltaSeconds :type Float%20%28single-precision%29)))

(event Input|ActionEvents|InputActionSetDestination
  (params (Key :type Key%20Structure :default "None"))
  (bind _box_carrier (Variables|Default|GetBox%20Carrier))
  ;[1 0.9508 0.3787] LMB Action
  (:Pressed
    ;;[1 1 1] Detect double tap.
    (CallFunction|DetectDouble)
    ;;[0.2542 0.1356 0.4072] Hide all options on Input Action.
    (bind _outactors (Actor|GetAllActorswithTag "CanToggle"))
    (for _array_element _outactors
      (for _array_element_2 (Actor|GetComponentsbyTag _array_element "/Script/UMG.WidgetComponent" "Options")
        (Rendering|SetVisibility _array_element_2 false false)))
    ;;[1 1 1] If double tap Sprint else Walk
    (Variables|/Script/Engine.CharacterMovementComponent|SetMaxWalkSpeed (Variables|/Script/Engine.Character|GetCharacterMovement _box_carrier) (Math|Float|SelectFloat (Variables|Default|GetSprintSpeed) (Variables|Default|GetWalkSpeed) (Variables|Default|GetbIsSprint)))
    (Class|BPIPlayerCommands|MovetoLocationLMB(Message) _box_carrier (.Location (Collision|BreakHitResult (.HitResult (Game|Player|GetHitResultUnderCursorbyChannel "TraceTypeQuery1" true))))))
  (:Released
    (Variables|Default|SetDoubleTap_Timer (Utilities|Time|GetTimeSeconds))))

(event Input|ActionEvents|InputActionToggle
  (params (Key :type Key%20Structure :default "None"))
  (bind (_hitresult _returnvalue) (Game|Player|GetHitResultUnderCursorbyChannel "TraceTypeQuery4" true))
  (bind _hitactor (Collision|BreakHitResult _hitresult))
  ;[1 0.9962 0.4444] RMB Action
  (:Pressed
    ;;[0.1046 0.05613 0.1683] Hide all options on Input Action.
    (bind _outactors (Actor|GetAllActorswithTag "CanToggle"))
    (for _array_element _outactors
      (for _array_element_2 (Actor|GetComponentsbyTag _array_element "/Script/UMG.WidgetComponent" "Options")
        (Rendering|SetVisibility _array_element_2 false false)))
    (if _returnvalue
      (if (Utilities|DoesObjectImplementInterface _hitactor "/Game/Actors/Interfaces/BPI_CanToggle.BPI_CanToggle_C")
        (Class|BPICanToggle|ToggleVisibility(Message) _hitactor)))))

(fn ConstructionScript)

(fn DetectDouble
  (Variables|Default|SetbIsSprint (< (- (Utilities|Time|GetTimeSeconds) (Variables|Default|GetDoubleTap_Timer)) (Variables|Default|GetDoubleTapSpeed))))