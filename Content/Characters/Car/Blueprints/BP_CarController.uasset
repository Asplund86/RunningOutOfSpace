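; BP_CarController is a traffic manager that spawns BP_Car actors, has them throw pickups and removes them.
; On BeginPlay it starts a looping SpawnCar timer with an interval randomized once, and offsets the spawn point and two triggers from its own location.
; Overlapping cars are identified through BPI_Car: ThrowActivater sends ThrowPickupMessage with a random value, and Destroyer destroys them.
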(event OnComponentBeginOverlap(ThrowActivater)
  (params (OverlappedComponent :type Primitive%20Component%20Object%20Reference) (OtherActor :type Actor%20Object%20Reference) (OtherComp :type Primitive%20Component%20Object%20Reference) (OtherBodyIndex :type Integer) (bFromSweep :type Boolean) (SweepResult :type Hit%20Result%20Structure%20%28by%20ref%29))
  (if (Utilities|DoesObjectImplementInterface OtherActor "/Game/Characters/Car/Blueprints/BPI_CAr.BPI_Car_C")
    (Class|BPICar|ThrowPickup(Message) OtherActor (Math|Random|RandomFloatinRange -1.1e+04 -1.7e+04))))

(event OnComponentBeginOverlap(Destroyer)
  (params (OverlappedComponent :type Primitive%20Component%20Object%20Reference) (OtherActor :type Actor%20Object%20Reference) (OtherComp :type Primitive%20Component%20Object%20Reference) (OtherBodyIndex :type Integer) (bFromSweep :type Boolean) (SweepResult :type Hit%20Result%20Structure%20%28by%20ref%29))
  (if (Utilities|DoesObjectImplementInterface OtherActor "/Game/Characters/Car/Blueprints/BPI_CAr.BPI_Car_C")
    (Actor|DestroyActor OtherActor)))

(event EventBeginPlay
  (Variables|Default|SetSpawnCarLocation (+ (Transformation|GetActorLocation) (Variables|Default|GetSpawnCarLocation)))
  (Utilities|Time|SetTimerbyFunctionName 0 "SpawnCar" (Math|Random|RandomFloatinRange 5.0 2e+01) true -9.0)
  (Transformation|SetWorldLocation (Variables|Default|GetThrowActivater) (+ (Transformation|GetActorLocation) (Variables|Default|GetThrowActivaterLocation)) false false)
  (Transformation|SetWorldLocation (Variables|Default|GetDestroyer) (+ (Transformation|GetActorLocation) (Variables|Default|GetDestroyerLocation)) false false))

(event Collision|EventActorBeginOverlap
  (params (OtherActor :type Actor%20Object%20Reference)))

(event EventTick
  (params (DeltaSeconds :type Float%20%28single-precision%29)))

(fn ConstructionScript)

(fn SpawnCar
  (bind _returnvalue (Game|SpawnActorfromClass "/Game/Characters/Car/Blueprints/BP_Car.BP_Car_C" (Math|Transform|MakeTransform (Variables|Default|GetSpawnCarLocation) "0.000000,90.000000, 0" "1,1,1") "AlwaysSpawn" 0 0))
  (Variables|Default|SetCar _returnvalue))