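; BP_Car is a car actor that drives forward on its own and can throw pickups.
; On BeginPlay it writes a random vector to the mesh's custom primitive data, giving per-instance variation, and Tick offsets it by Velocity without sweep or delta-time scaling.
; ThrowPickup waits up to a second, spawns a BP_Pickup at SpawnPickupPoint and launches it with the passed X impulse plus random sideways and upward force.
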(event EventBeginPlay
  (Rendering|Material|SetCustomPrimitiveDataVector3 (Variables|Default|GetCarMesh) 0 (Math|Vector|MakeVector (Math|Random|RandomFloat) (Math|Random|RandomFloat) (Math|Random|RandomFloat))))

(event Collision|EventActorBeginOverlap
  (params (OtherActor :type Actor%20Object%20Reference)))

(event EventTick
  (params (DeltaSeconds :type Float%20%28single-precision%29))
  ;[1 1 1] Move the car
  (Transformation|AddActorWorldOffset (* (Transformation|GetActorForwardVector) (Variables|Default|GetVelocity))))

(event EventThrowPickup
  (params (Velocity :type Float%20%28single-precision%29))
  (Utilities|FlowControl|Delay (Math|Random|RandomFloatinRange 0.0 1.0))
  (bind _returnvalue (Game|SpawnActorfromClass "/Game/Actors/Pickups/Blueprints/BP_Pickup.BP_Pickup_C" (Transformation|GetWorldTransform (Variables|Default|GetSpawnPickupPoint)) "AlwaysSpawn" 0 0))
  (Physics|AddImpulse (Variables|/Game/Actors/Pickups/Blueprints/BP_Pickup.BP_Pickup_C|GetMesh _returnvalue) (Math|Vector|MakeVector Velocity (Math|Random|RandomFloatinRange -5e+03 5e+03) (Math|Random|RandomFloatinRange 7e+03 8e+03)) "None" false))

(fn ConstructionScript)