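; BP_Player is the player Blueprint, providing move-to navigation and the beginnings of a physics-based pickup.
; Its events send the cached PlayerController to a location or actor through SimpleMoveTo calls.
; InitiatePickup starts a move to the target and immediately calls Pickup, which is an empty stub with an unconnected distance check.
; Tick keeps the PhysicsHandle target at the GrabLocation component's world position.
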(event EventBeginPlay
  (Variables|Default|SetPlayer_Controller (Game|GetPlayerController 0)))

(event Collision|EventActorBeginOverlap
  (params (OtherActor :type Actor%20Object%20Reference)))

(event EventTick
  (params (DeltaSeconds :type Float%20%28single-precision%29))
  (Physics|Components|PhysicsHandle|SetTargetLocation (Variables|Default|GetPhysicsHandle) (Transformation|GetWorldLocation (Variables|Default|GetGrabLocation))))

(event EventInitiatePickup
  (params (TargetActor :type Actor%20Object%20Reference) (TargetComponent :type Primitive%20Component%20Object%20Reference))
  (AI|Navigation|SimpleMovetoActor (Variables|Default|GetPlayer_Controller) TargetActor)
  (CallFunction|Pickup TargetComponent))

(event EventMovetoLocation
  (params (Location :type Vector :default "0, 0, 0"))
  (AI|Navigation|SimpleMovetoLocation (Variables|Default|GetPlayer_Controller) Location))

(event EventMovetoActor
  (params (Actor :type Actor%20Object%20Reference))
  (AI|Navigation|SimpleMovetoActor (Variables|Default|GetPlayer_Controller) Actor))

(fn ConstructionScript)

(fn Pickup
  (params (TargetComponent :type Primitive%20Component%20Object%20Reference)))