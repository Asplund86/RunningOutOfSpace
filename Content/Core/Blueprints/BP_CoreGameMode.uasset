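; BP_CoreGameMode is a game mode Blueprint that tracks a running score against a win target.
; BeginPlay sets the target, and the ScoreAmount event adds incoming points to the total.
; A separate CheckifScore event, when passed true, prints the total and a win message if the target is reached.
; The win is only a debug print, with no further game-ending logic.
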(event EventBeginPlay
  (Variables|Default|SetScoreToWin 30))

(event EventTick
  (params (DeltaSeconds :type Float%20%28single-precision%29)))

(event EventCheckifScore
  (params (bIsScore? :type Boolean))
  (bind _totalscore (Variables|Default|GetTotalScore))
  (if bIsScore?
    (Development|PrintString (Utilities|String|ToString(Integer) _totalscore))
    (if (>= _totalscore (Variables|Default|GetScoreToWin))
      (Development|PrintString "WIN!"))))

(event EventScoreAmount
  (params (Score :type Integer))
  (Variables|Default|SetTotalScore (+ Score (Variables|Default|GetTotalScore))))

(fn ConstructionScript)