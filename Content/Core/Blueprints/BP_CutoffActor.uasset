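; BP_CutoffActor is a placeable actor that drives a cutoff effect through the MPC_Cutoff material parameter collection.
; It writes its root's world position, a fringe color, and radius, power, hardness and boost values into the collection.
; The same writes run in the construction script and on BeginPlay, with no Tick update, so movement during play is not tracked.
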(event EventBeginPlay
  (Rendering|Material|SetVectorParameterValue "/Game/Core/Materials/Collection/MPC_Cutoff.MPC_Cutoff" "CustomPosition" (Math|Conversions|ToLinearColor(Vector) (Transformation|GetWorldLocation (Variables|Default|GetDefaultSceneRoot))) :!class /Script/Engine.KismetMaterialLibrary)
  (Rendering|Material|SetVectorParameterValue "/Game/Core/Materials/Collection/MPC_Cutoff.MPC_Cutoff" "FringeColor" (Variables|Default|GetFridngeColor) :!class /Script/Engine.KismetMaterialLibrary)
  (Rendering|Material|SetScalarParameterValue "/Game/Core/Materials/Collection/MPC_Cutoff.MPC_Cutoff" "Radius" (Variables|Default|GetRadius) :!class /Script/Engine.KismetMaterialLibrary)
  (Rendering|Material|SetScalarParameterValue "/Game/Core/Materials/Collection/MPC_Cutoff.MPC_Cutoff" "Power" (Variables|Default|GetPower) :!class /Script/Engine.KismetMaterialLibrary)
  (Rendering|Material|SetScalarParameterValue "/Game/Core/Materials/Collection/MPC_Cutoff.MPC_Cutoff" "Hardness" (Variables|Default|GetHardness) :!class /Script/Engine.KismetMaterialLibrary)
  (Rendering|Material|SetScalarParameterValue "/Game/Core/Materials/Collection/MPC_Cutoff.MPC_Cutoff" "Boost" (Variables|Default|GetBoost) :!class /Script/Engine.KismetMaterialLibrary))

(event Collision|EventActorBeginOverlap
  (params (OtherActor :type Actor%20Object%20Reference)))

(event EventTick
  (params (DeltaSeconds :type Float%20%28single-precision%29)))

(fn ConstructionScript
  (Rendering|Material|SetVectorParameterValue "/Game/Core/Materials/Collection/MPC_Cutoff.MPC_Cutoff" "CustomPosition" (Math|Conversions|ToLinearColor(Vector) (Transformation|GetWorldLocation (Variables|Default|GetDefaultSceneRoot))) :!class /Script/Engine.KismetMaterialLibrary)
  (Rendering|Material|SetVectorParameterValue "/Game/Core/Materials/Collection/MPC_Cutoff.MPC_Cutoff" "FringeColor" (Variables|Default|GetFridngeColor) :!class /Script/Engine.KismetMaterialLibrary)
  (Rendering|Material|SetScalarParameterValue "/Game/Core/Materials/Collection/MPC_Cutoff.MPC_Cutoff" "Radius" (Variables|Default|GetRadius) :!class /Script/Engine.KismetMaterialLibrary)
  (Rendering|Material|SetScalarParameterValue "/Game/Core/Materials/Collection/MPC_Cutoff.MPC_Cutoff" "Power" (Variables|Default|GetPower) :!class /Script/Engine.KismetMaterialLibrary)
  (Rendering|Material|SetScalarParameterValue "/Game/Core/Materials/Collection/MPC_Cutoff.MPC_Cutoff" "Hardness" (Variables|Default|GetHardness) :!class /Script/Engine.KismetMaterialLibrary)
  (Rendering|Material|SetScalarParameterValue "/Game/Core/Materials/Collection/MPC_Cutoff.MPC_Cutoff" "Boost" (Variables|Default|GetBoost) :!class /Script/Engine.KismetMaterialLibrary))